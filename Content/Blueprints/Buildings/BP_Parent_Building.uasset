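; Parent building Blueprint that recolors exterior walls, interior walls, floors, curtains and terraces from per-building color variables.
; Its construction script creates one dynamic material instance per surface type, sets its color parameters, and also feeds BuildingAge into the exterior wall mask.
; Each instance is applied to the static mesh children of its grouping component, by slot index or by the Interior and Terrace slot names.
; The event graph holds no runtime logic.
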(event EventBeginPlay)

(event Collision|EventActorBeginOverlap
  (params (OtherActor :type Actor%20Object%20Reference)))

(event EventTick
  (params (DeltaSeconds :type Float%20%28single-precision%29)))

(fn ConstructionScript
  ;[1 1 1] Set Exterior Wall Colors
  (bind _returnvalue (Rendering|Material|CreateDynamicMaterialInstance (Variables|Default|GetExteriorWallMat) "None" "None" :!class /Script/Engine.KismetMaterialLibrary))
  (bind _output_get (Variables|Default|SetBuildingExtWallMatInst _returnvalue))
  (Rendering|Material|SetVectorParameterValue _output_get "PaintColor" (Variables|Default|GetExteriorWallPaint1) :!class /Script/Engine.MaterialInstanceDynamic)
  (Rendering|Material|SetVectorParameterValue (Variables|Default|GetBuildingExtWallMatInst) "PaintColor2" (Variables|Default|GetExteriorWallPaint2) :!class /Script/Engine.MaterialInstanceDynamic)
  (Rendering|Material|SetScalarParameterValue (Variables|Default|GetBuildingExtWallMatInst) "WMaskMultiplier" (Variables|Default|GetBuildingAge) :!class /Script/Engine.MaterialInstanceDynamic)
  (for _array_element (Components|GetChildrenComponents (Variables|Default|GetWalls) false)
    (bind _asstatic_mesh_component (Utilities|Casting|CastToStaticMeshComponent _array_element))
    (Rendering|Material|SetMaterial _asstatic_mesh_component 0 (Variables|Default|GetBuildingExtWallMatInst)))
  ;[1 1 1] Set Interior Wall Color
  (bind _returnvalue_2 (Rendering|Material|CreateDynamicMaterialInstance (Variables|Default|GetInteriorWallMat) "None" "None" :!class /Script/Engine.KismetMaterialLibrary))
  (bind _output_get_2 (Variables|Default|SetBuildingIntWallInst _returnvalue_2))
  (Rendering|Material|SetVectorParameterValue _output_get_2 "WallpaperColor" (Variables|Default|GetInteriorWallColor) :!class /Script/Engine.MaterialInstanceDynamic)
  (for _array_element_2 (Components|GetChildrenComponents (Variables|Default|GetWalls) false)
    (bind _asstatic_mesh_component_2 (Utilities|Casting|CastToStaticMeshComponent _array_element_2))
    (Rendering|Material|SetMaterialbyName _asstatic_mesh_component_2 "Interior" (Variables|Default|GetBuildingIntWallInst)))
  (for _array_element_3 (Components|GetChildrenComponents (Variables|Default|GetInteriorWalls) false)
    (bind _asstatic_mesh_component_3 (Utilities|Casting|CastToStaticMeshComponent _array_element_3))
    (Rendering|Material|SetMaterialbyName _asstatic_mesh_component_3 "Interior" (Variables|Default|GetBuildingIntWallInst)))
  ;[1 1 1] Set Floor Color
  (bind _returnvalue_3 (Rendering|Material|CreateDynamicMaterialInstance (Variables|Default|GetFloorMat) "None" "None" :!class /Script/Engine.KismetMaterialLibrary))
  (bind _output_get_3 (Variables|Default|SetBuildingIntFloorInst _returnvalue_3))
  (Rendering|Material|SetVectorParameterValue _output_get_3 "FloorColor" (Variables|Default|GetFloorColor) :!class /Script/Engine.MaterialInstanceDynamic)
  (for _array_element_4 (Components|GetChildrenComponents (Variables|Default|GetFloors) false)
    (bind _asstatic_mesh_component_4 (Utilities|Casting|CastToStaticMeshComponent _array_element_4))
    (Rendering|Material|SetMaterial _asstatic_mesh_component_4 0 (Variables|Default|GetBuildingIntFloorInst)))
  ;[1 1 1] Set Curtain Colors
  (bind _returnvalue_4 (Rendering|Material|CreateDynamicMaterialInstance (Variables|Default|GetCurtainMat) "None" "None" :!class /Script/Engine.KismetMaterialLibrary))
  (bind _output_get_4 (Variables|Default|SetCurtainInst _returnvalue_4))
  (Rendering|Material|SetVectorParameterValue _output_get_4 "CurtainColor" (Variables|Default|GetCurtainColor) :!class /Script/Engine.MaterialInstanceDynamic)
  (for _array_element_5 (Components|GetChildrenComponents (Variables|Default|GetCurtains) false)
    (bind _asstatic_mesh_component_5 (Utilities|Casting|CastToStaticMeshComponent _array_element_5))
    (Rendering|Material|SetMaterial _asstatic_mesh_component_5 0 (Variables|Default|GetCurtainInst)))
  ;[1 1 1] Set Terrace Colors
  (bind _returnvalue_5 (Rendering|Material|CreateDynamicMaterialInstance "/Game/Maps/WesterTown/Materials/Structure/Exterior/M_Building_Terrace.M_Building_Terrace" "" "None" :!class /Script/Engine.KismetMaterialLibrary))
  (bind _output_get_5 (Variables|Default|SetTerraceInst _returnvalue_5))
  (Rendering|Material|SetVectorParameterValue _output_get_5 "TerraceColor" (Variables|Default|GetTerraceColor) :!class /Script/Engine.MaterialInstanceDynamic)
  (for _array_element_6 (Components|GetChildrenComponents (Variables|Default|GetTerrace) false)
    (bind _asstatic_mesh_component_6 (Utilities|Casting|CastToStaticMeshComponent _array_element_6))
    (Rendering|Material|SetMaterialbyName _asstatic_mesh_component_6 "Terrace" (Variables|Default|GetTerraceInst))))