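; BP_Sky is a sky sphere Blueprint whose material follows a directional light to represent the sun.
; The construction script creates a dynamic material instance on SkySphereMesh as SkyMaterial, while BeginPlay creates one stored separately as SphereMaterial.
; UpdateSunDirection pushes the light actor's forward vector and color into SkyMaterial's light direction and sun color parameters.
; Nothing in these graphs calls UpdateSunDirection.
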(event EventBeginPlay
  (bind _returnvalue (Rendering|Material|CreateDynamicMaterialInstance (Variables|BP_Skydome|GetSky%20Sphere%20mesh) 0 0 "None" :!class /Script/Engine.PrimitiveComponent))
  (Variables|Default|SetSphereMaterial _returnvalue))

(fn ConstructionScript
  (bind _returnvalue (Rendering|Material|CreateDynamicMaterialInstance (Variables|BP_Skydome|GetSky%20Sphere%20mesh) 0 0 "None" :!class /Script/Engine.PrimitiveComponent))
  (Variables|Default|SetSky%20material _returnvalue))

(fn UpdateSunDirection
  (bind _sky_material (Variables|Default|GetSky%20material))
  (Rendering|Material|SetVectorParameterValue _sky_material "Light direction" (Math|Conversions|ToLinearColor(Vector) (Math|Rotator|GetRotationXVector (Transformation|GetActorRotation (Variables|Default|GetDirectional%20light%20actor)))) :!class /Script/Engine.MaterialInstanceDynamic)
  (Rendering|Material|SetVectorParameterValue _sky_material "Sun color" (Math|Conversions|ToLinearColor(Color) (Variables|/Script/Engine.LightComponentBase|GetLightColor (Variables|/Script/Engine.Light|GetLightComponent (Variables|Default|GetDirectional%20light%20actor)))) :!class /Script/Engine.MaterialInstanceDynamic))